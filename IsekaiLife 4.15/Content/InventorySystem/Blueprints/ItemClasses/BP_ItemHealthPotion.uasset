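; BP_ItemHealthPotion is an inventory item actor that restores health to the character when used.
; On OnUsed, it checks the owning character's CurrentHP against MaxHP through InventoryRef, and if below, adds HPadd health and removes one unit at its inventory Index.
; The actor destroys itself in either case, so at full health the potion stays in the inventory.
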(event EventBeginPlay)

(event Collision|EventActorBeginOverlap
  (params (OtherActor :type Actor%20Object%20Reference)))

(event EventTick
  (params (DeltaSeconds :type Float%20%28single-precision%29)))

(event EventOnUsed
  (bind _inventoryref (Variables|Default|GetInventoryRef))
  (bind _mycharacterref (Variables|/Game/InventorySystem/Blueprints/BP_Inventory.BP_Inventory_C|GetMyCharacterRef _inventoryref))
  (if (< (Variables|/Game/Game/Character/Player/Ch_MyCharacter.Ch_MyCharacter_C|GetCurrentHP _mycharacterref) (Variables|/Game/Game/Character/Player/Ch_MyCharacter.Ch_MyCharacter_C|GetMaxHP _mycharacterref))
    (Default|IncreaseHealth _mycharacterref (Variables|Default|GetHPadd))
    (Default|RemoveItematIndex (Variables|Default|GetInventoryRef) (Variables|Default|GetIndex) 1)
    (Actor|DestroyActor)
    (else
      (Actor|DestroyActor))))

(fn ConstructionScript
  (|CallParentFunction))