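; World pickup actor that adds an item class and amount to the player's inventory when picked up.
; Its sphere overlap queues it in the character's nearby pickup list, and only the first entry shows its name and amount widget.
; Pickup keeps any amount that did not fit, records the remainder by ID in the inventory's looted list, and destroys the actor once empty.
; Leaving or emptying hands the prompt to the next queued pickup.
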(event OnComponentBeginOverlap(Sphere)
  (params (OverlappedComponent :type Primitive%20Component%20Object%20Reference) (OtherActor :type Actor%20Object%20Reference) (OtherComp :type Primitive%20Component%20Object%20Reference) (OtherBodyIndex :type Integer) (bFromSweep :type Boolean) (SweepResult :type Hit%20Result%20Structure%20%28by%20ref%29))
  (bind _asch_my_character (Utilities|Casting|CastToCh_MyCharacter OtherActor))
  (if (> (Utilities|Array|Length (Variables|/Game/Game/Character/Player/Ch_MyCharacter.Ch_MyCharacter_C|GetNearbyPickupActor _asch_my_character)) 0)
    (Utilities|Array|Add (Variables|/Game/Game/Character/Player/Ch_MyCharacter.Ch_MyCharacter_C|GetNearbyPickupActor _asch_my_character) self)
    (else
      (Rendering|SetVisibility (Variables|Default|GetPickUpText) true false)
      (Utilities|Array|Add (Variables|/Game/Game/Character/Player/Ch_MyCharacter.Ch_MyCharacter_C|GetNearbyPickupActor _asch_my_character) self))))

(event OnComponentEndOverlap(Sphere)
  (params (OverlappedComponent :type Primitive%20Component%20Object%20Reference) (OtherActor :type Actor%20Object%20Reference) (OtherComp :type Primitive%20Component%20Object%20Reference) (OtherBodyIndex :type Integer))
  (bind _asch_my_character (Utilities|Casting|CastToCh_MyCharacter OtherActor))
  (if (and (Utilities|IsValid (Utilities|Array|Get(acopy) (Variables|/Game/Game/Character/Player/Ch_MyCharacter.Ch_MyCharacter_C|GetNearbyPickupActor _asch_my_character))) (== (Utilities|Array|Get(acopy) (Variables|/Game/Game/Character/Player/Ch_MyCharacter.Ch_MyCharacter_C|GetNearbyPickupActor _asch_my_character)) self))
    (Rendering|SetVisibility (Variables|Default|GetPickUpText) false false)
    (Utilities|Array|RemoveItem (Variables|/Game/Game/Character/Player/Ch_MyCharacter.Ch_MyCharacter_C|GetNearbyPickupActor _asch_my_character) self)
    (Utilities|IsValid (Utilities|Array|Get(acopy) (Variables|/Game/Game/Character/Player/Ch_MyCharacter.Ch_MyCharacter_C|GetNearbyPickupActor _asch_my_character))
      (:Is%20Valid
        (Rendering|SetVisibility (Variables|BP_PickUpActor_C|GetPickUpText (Utilities|Array|Get(acopy) (Variables|/Game/Game/Character/Player/Ch_MyCharacter.Ch_MyCharacter_C|GetNearbyPickupActor _asch_my_character))) true false)))
    (else
      (Utilities|Array|RemoveItem (Variables|/Game/Game/Character/Player/Ch_MyCharacter.Ch_MyCharacter_C|GetNearbyPickupActor _asch_my_character) self))))

(event Custom|OnPickedUp
  (params (MyCharacter :type Ch%20My%20Character%20Object%20Reference))
  (bind _inventoryref (Variables|/Game/Game/Character/Player/Ch_MyCharacter.Ch_MyCharacter_C|GetInventoryRef MyCharacter))
  (bind _nearbypickupactor (Variables|/Game/Game/Character/Player/Ch_MyCharacter.Ch_MyCharacter_C|GetNearbyPickupActor MyCharacter))
  (bind _inventoryref_2 (Variables|/Game/Game/Character/Player/Ch_MyCharacter.Ch_MyCharacter_C|GetInventoryRef MyCharacter))
  (bind _item (Utilities|Array|Get(acopy) _nearbypickupactor))
  (Utilities|IsValid _inventoryref
    (:Is%20Valid
      (bind (_success_ _rest) (Default|AddItem _inventoryref (Variables|Default|GetItemToAdd) (Variables|Default|GetAmount) true))
      (if _success_
        (if (> _rest 0)
          (Variables|Default|SetAmount _rest)
          (CallFunction|UpdateText)
          (Utilities|Array|Add (Variables|/Game/InventorySystem/Blueprints/BP_Inventory.BP_Inventory_C|GetLootedPickups _inventoryref_2) (Utilities|Struct|MakeS_SavedPickup (Variables|Default|GetID) (Variables|Default|GetAmount)))
          (else
            (Utilities|Array|Add (Variables|/Game/InventorySystem/Blueprints/BP_Inventory.BP_Inventory_C|GetLootedPickups _inventoryref_2) (Utilities|Struct|MakeS_SavedPickup (Variables|Default|GetID) 0))
            (Utilities|Array|RemoveItem _nearbypickupactor self)
            (Utilities|IsValid _item
              (:Is%20Valid
                (Rendering|SetVisibility (Variables|BP_PickUpActor_C|GetPickUpText _item) true false)
                (Actor|DestroyActor))
              (:Is%20Not%20Valid
                (Actor|DestroyActor)))))))))

(event EventBeginPlay
  (CallFunction|UpdateText))

(fn ConstructionScript)

(fn UpdateText
  (bind _aspickup_text (Utilities|Casting|CastToPickupText (UserInterface|GetUserWidgetObject (Variables|Default|GetPickUpText)))
    (:then
      (Rendering|Components|TextRender|SetText (Variables|/Game/InventorySystem/Widgets/PickupText.PickupText_C|GetNameText _aspickup_text) (Utilities|Text|FormatText "{Name} ({Amount})" (.Name (Utilities|Struct|BreakS_ItemInfo (.ItemInfo (Utilities|GetClassDefaults (Variables|Default|GetItemToAdd))))) (Utilities|Text|ToText(Integer) (Variables|Default|GetAmount)))))
    (:CastFailed
      _))
  (return))