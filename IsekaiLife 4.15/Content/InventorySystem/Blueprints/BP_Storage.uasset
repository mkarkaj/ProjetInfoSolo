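; Storage container actor for the inventory system, holding a fixed number of item slots seeded from a starting item list.
; Slot functions add, remove, swap and merge stacks, with AddItem recursing to spread overflow across free stacks and empty slots.
; Items move in from a player inventory slot or all out at once.
; Changes refresh the storage widget taken from the player's inventory UI, and show/hide toggles input mode and cursor.
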(event Custom|UpdateSlotAtIndex
  (params (Index :type Integer))
  (Default|UpdateSlot (Utilities|Array|Get(acopy) (Variables|/Game/InventorySystem/Widgets/StorageWidget.StorageWidget_C|GetSlotsWidgets (Variables|Default|GetStorageWidget)) Index)))

(event Collision|EventActorBeginOverlap
  (params (OtherActor :type Actor%20Object%20Reference)))

(event EventTick
  (params (DeltaSeconds :type Float%20%28single-precision%29)))

(event EventBeginPlay
  (Variables|Item|SetSlots (Variables|Default|GetStartItem))
  (Variables|Default|SetStorageWidget (Variables|/Game/Game/Widget/MainWidget.MainWidget_C|GetStorageWidget_216 (Variables|/Game/InventorySystem/Blueprints/BP_Inventory.BP_Inventory_C|GetMainWidget (Variables|/Game/Game/Character/Player/Ch_MyCharacter.Ch_MyCharacter_C|GetInventoryRef (Variables|Default|GetMyCharacterRef)))))
  (Utilities|Array|Resize (Variables|Item|GetSlots) (Variables|Inventory|GetAmountOfSlots)))

(fn ConstructionScript)

(fn IsSlotEmpty?
  (params (Index :type Integer))
  (return (not (Utilities|IsValidClass (.ItemClass (Utilities|Struct|BreakS_InventorySlot (Utilities|Array|Get(acopy) (Variables|Item|GetSlots) Index)))))))

(fn GetItemInfoatIndex
  (params (Index :type Integer))
  (bind _slots (Variables|Item|GetSlots))
  (bind _item (Utilities|Array|Get(acopy) _slots Index))
  (bind (_itemclass _amount) (Utilities|Struct|BreakS_InventorySlot _item))
  (if (Utilities|IsValidClass _itemclass)
    (return false (.ItemInfo (Utilities|GetClassDefaults _itemclass)) _amount)
    (else
      (return true "" 0))))

(fn SearchEmptySlot
  (bind (_array_element _array_index) (Utilities|Array|ForEachLoopwithBreak (Variables|Item|GetSlots) :!label _label)
    (:LoopBody
      (if (not (Utilities|IsValidClass (.ItemClass (Utilities|Struct|BreakS_InventorySlot _array_element))))
        (LocalVariables|SetLocalBool true)
        (LocalVariables|SetLocalIndex _array_index)
        (goto _label Break)))
    (:Completed
      (return (LocalVariables|GetLocalBool) (LocalVariables|GetLocalIndex)))))

(fn SearchFreeStack
  (params (ItemClass :type BP%20Master%20Item%20Class%20Reference))
  (bind (_array_element _array_index) (Utilities|Array|ForEachLoopwithBreak (Variables|Item|GetSlots) :!label _label)
    (:LoopBody
      (if (Utilities|IsValidClass (.ItemClass (Utilities|Struct|BreakS_InventorySlot _array_element)))
        (if (and (== (.ItemClass (Utilities|Struct|BreakS_InventorySlot _array_element)) ItemClass) (< (.Amount (Utilities|Struct|BreakS_InventorySlot _array_element)) (Variables|Item|GetMaxStackSize)))
          (LocalVariables|SetLocalBool true)
          (LocalVariables|SetLocalIndex _array_index)
          (goto _label Break))))
    (:Completed
      (return (LocalVariables|GetLocalBool) (LocalVariables|GetLocalIndex)))))

(fn GetAmountatIndex
  (params (Index :type Integer))
  (return (.Amount (Utilities|Struct|BreakS_InventorySlot (Utilities|Array|Get(acopy) (Variables|Item|GetSlots) Index)))))

(fn RemoveItematIndex
  (params (Index :type Integer) (Amount :type Integer))
  (bind _slots (Variables|Item|GetSlots))
  (LocalVariables|SetLocalIndex Index)
  (LocalVariables|SetLocalAmount Amount)
  (if (and (not (Inventory|IsSlotEmpty? (LocalVariables|GetLocalIndex))) (> (LocalVariables|GetLocalAmount) 0))
    (if (>= (LocalVariables|GetLocalAmount) (Item|GetAmountatIndex (LocalVariables|GetLocalIndex)))
      (Utilities|Array|SetArrayElem (Variables|Item|GetSlots) (LocalVariables|GetLocalIndex) "")
      (CallFunction|UpdateSlotatIndex (LocalVariables|GetLocalIndex))
      (return true)
      (else
        (Utilities|Array|SetArrayElem _slots (LocalVariables|GetLocalIndex) (Utilities|Struct|MakeS_InventorySlot (.ItemClass (Utilities|Struct|BreakS_InventorySlot (Utilities|Array|Get(acopy) _slots (LocalVariables|GetLocalIndex)))) (- (.Amount (Utilities|Struct|BreakS_InventorySlot (Utilities|Array|Get(acopy) _slots (LocalVariables|GetLocalIndex)))) (LocalVariables|GetLocalAmount))))
        (CallFunction|UpdateSlotatIndex (LocalVariables|GetLocalIndex))
        (return true)))
    (else
      (return false))))

(fn SwapSlots
  (params (Index1 :type Integer) (Index2 :type Integer))
  (bind _slots (Variables|Item|GetSlots))
  (bind _returnvalue (Utilities|Array|LastIndex _slots))
  (LocalVariables|SetLocalIndex1 Index1)
  (LocalVariables|SetLocalIndex2 Index2)
  (if (or (> (LocalVariables|GetLocalIndex1) _returnvalue) (> (LocalVariables|GetLocalIndex2) _returnvalue))
    (return false)
    (else
      (LocalVariables|SetLocalSlot2 (Utilities|Array|Get(acopy) (Variables|Item|GetSlots) (LocalVariables|GetLocalIndex2)))
      (Utilities|Array|SetArrayElem (Variables|Item|GetSlots) (LocalVariables|GetLocalIndex2) (Utilities|Array|Get(acopy) (Variables|Item|GetSlots) (LocalVariables|GetLocalIndex1)))
      (Utilities|Array|SetArrayElem (Variables|Item|GetSlots) (LocalVariables|GetLocalIndex1) (LocalVariables|GetLocalSlot2))
      (CallFunction|UpdateSlotatIndex (LocalVariables|GetLocalIndex1))
      (CallFunction|UpdateSlotatIndex (LocalVariables|GetLocalIndex2))
      (return true))))

(fn AddtoIndex
  (params (FromIndex :type Integer) (ToIndex :type Integer))
  (LocalVariables|SetLocalFrom FromIndex)
  (LocalVariables|SetLocalTo ToIndex)
  (if (Math|Boolean|ANDBoolean (== (.ItemClass (Utilities|Struct|BreakS_InventorySlot (Utilities|Array|Get(acopy) (Variables|Item|GetSlots) (LocalVariables|GetLocalFrom)))) (.ItemClass (Utilities|Struct|BreakS_InventorySlot (Utilities|Array|Get(acopy) (Variables|Item|GetSlots) (LocalVariables|GetLocalTo))))) (< (.Amount (Utilities|Struct|BreakS_InventorySlot (Utilities|Array|Get(acopy) (Variables|Item|GetSlots) (LocalVariables|GetLocalTo)))) (Variables|Item|GetMaxStackSize)) (.CanBeStacked? (Utilities|Struct|BreakS_ItemInfo (.ItemInfo (Item|GetItemInfoatIndex (LocalVariables|GetLocalTo))))))
    (LocalVariables|SetLocalClass (.ItemClass (Utilities|Struct|BreakS_InventorySlot (Utilities|Array|Get(acopy) (Variables|Item|GetSlots) (LocalVariables|GetLocalFrom)))))
    (if (>= (- (Variables|Item|GetMaxStackSize) (Item|GetAmountatIndex (LocalVariables|GetLocalTo))) (Item|GetAmountatIndex (LocalVariables|GetLocalFrom)))
      (Utilities|Array|SetArrayElem (Variables|Item|GetSlots) (LocalVariables|GetLocalTo) (Utilities|Struct|MakeS_InventorySlot (LocalVariables|GetLocalClass) (+ (Item|GetAmountatIndex (LocalVariables|GetLocalTo)) (Item|GetAmountatIndex (LocalVariables|GetLocalFrom)))))
      (Utilities|Array|SetArrayElem (Variables|Item|GetSlots) (LocalVariables|GetLocalFrom) (Utilities|Struct|MakeS_InventorySlot 0 0))
      (else
        (Utilities|Array|SetArrayElem (Variables|Item|GetSlots) (LocalVariables|GetLocalFrom) (Utilities|Struct|MakeS_InventorySlot (LocalVariables|GetLocalClass) (- (Item|GetAmountatIndex (LocalVariables|GetLocalFrom)) (- (Variables|Item|GetMaxStackSize) (Item|GetAmountatIndex (LocalVariables|GetLocalTo))))))
        (Utilities|Array|SetArrayElem (Variables|Item|GetSlots) (LocalVariables|GetLocalTo) (Utilities|Struct|MakeS_InventorySlot (LocalVariables|GetLocalClass) (Variables|Item|GetMaxStackSize)))))
    (CallFunction|UpdateSlotatIndex (LocalVariables|GetLocalFrom))
    (CallFunction|UpdateSlotatIndex (LocalVariables|GetLocalTo))
    (return true)
    (else
      (return false))))

(fn AddItem
  (params (ItemClass :type BP%20Master%20Item%20Class%20Reference) (Amount :type Integer))
  (LocalVariables|SetLocalClass ItemClass)
  (LocalVariables|SetLocalAmount Amount)
  (if (.CanBeStacked? (Utilities|Struct|BreakS_ItemInfo (.ItemInfo (Utilities|GetClassDefaults ItemClass))))
    (bind (_success_ _index) (Inventory|SearchFreeStack (LocalVariables|GetLocalClass)))
    (if _success_
      (LocalVariables|SetFoundIndex _index)
      (if (> (+ (.Amount (Utilities|Struct|BreakS_InventorySlot (Utilities|Array|Get(acopy) (Variables|Item|GetSlots) (LocalVariables|GetFoundIndex)))) (LocalVariables|GetLocalAmount)) (Variables|Item|GetMaxStackSize))
        (LocalVariables|SetLocalAmount (- (+ (.Amount (Utilities|Struct|BreakS_InventorySlot (Utilities|Array|Get(acopy) (Variables|Item|GetSlots) (LocalVariables|GetFoundIndex)))) (LocalVariables|GetLocalAmount)) (Variables|Item|GetMaxStackSize)))
        (Utilities|Array|SetArrayElem (Variables|Item|GetSlots) (LocalVariables|GetFoundIndex) (Utilities|Struct|MakeS_InventorySlot (LocalVariables|GetLocalClass) (Variables|Item|GetMaxStackSize)))
        (CallFunction|UpdateSlotatIndex (LocalVariables|GetFoundIndex))
        (bind (_success__2 _rest) (Item|AddItem (LocalVariables|GetLocalClass) (LocalVariables|GetLocalAmount)))
        (return _success__2 _rest)
        (else
          (Utilities|Array|SetArrayElem (Variables|Item|GetSlots) (LocalVariables|GetFoundIndex) (Utilities|Struct|MakeS_InventorySlot (LocalVariables|GetLocalClass) (+ (.Amount (Utilities|Struct|BreakS_InventorySlot (Utilities|Array|Get(acopy) (Variables|Item|GetSlots) (LocalVariables|GetFoundIndex)))) (LocalVariables|GetLocalAmount))))
          (CallFunction|UpdateSlotatIndex (LocalVariables|GetFoundIndex))
          (return true 0)))
      (else
        (bind (_success__3 _index_2) (Inventory|SearchEmptySlot))
        (if _success__3
          (LocalVariables|SetFoundIndex _index_2)
          (if (> (LocalVariables|GetLocalAmount) (Variables|Item|GetMaxStackSize))
            (Utilities|Array|SetArrayElem (Variables|Item|GetSlots) _index_2 (Utilities|Struct|MakeS_InventorySlot (LocalVariables|GetLocalClass) (Variables|Item|GetMaxStackSize)))
            (CallFunction|UpdateSlotatIndex (LocalVariables|GetFoundIndex))
            (bind (_success__4 _rest_2) (Item|AddItem (LocalVariables|GetLocalClass) (- (LocalVariables|GetLocalAmount) (Variables|Item|GetMaxStackSize))))
            (return _success__4 _rest_2)
            (else
              (Utilities|Array|SetArrayElem (Variables|Item|GetSlots) (LocalVariables|GetFoundIndex) (Utilities|Struct|MakeS_InventorySlot (LocalVariables|GetLocalClass) (LocalVariables|GetLocalAmount)))
              (CallFunction|UpdateSlotatIndex (LocalVariables|GetFoundIndex))
              (return true 0)))
          (else
            (return false (LocalVariables|GetLocalAmount))))))
    (else
      (bind (_success__5 _index_3) (Inventory|SearchEmptySlot))
      (if _success__5
        (bind _output_get (LocalVariables|SetFoundIndex _index_3))
        (Utilities|Array|SetArrayElem (Variables|Item|GetSlots) _output_get (Utilities|Struct|MakeS_InventorySlot (LocalVariables|GetLocalClass) 1))
        (CallFunction|UpdateSlotatIndex (LocalVariables|GetFoundIndex))
        (if (> (LocalVariables|GetLocalAmount) 1)
          (bind (_success__6 _rest_3) (Item|AddItem (LocalVariables|GetLocalClass) (- (LocalVariables|GetLocalAmount) 1)))
          (return _success__6 _rest_3)
          (else
            (return true 0)))
        (else
          (return false (LocalVariables|GetLocalAmount)))))))

(fn AddItemtoIndex
  (params (Index :type Integer) (ItemClass :type BP%20Master%20Item%20Class%20Reference) (Amount :type Integer))
  (if (and (Inventory|IsSlotEmpty? Index) (<= Amount (Variables|Item|GetMaxStackSize)))
    (Utilities|Array|SetArrayElem (Variables|Item|GetSlots) Index (Utilities|Struct|MakeS_InventorySlot ItemClass Amount))
    (CallFunction|UpdateSlotatIndex Index)
    (return true)
    (else
      (return false))))

(fn IncreaseAmountatIndex
  (params (Index :type Integer) (Amount :type Integer))
  (bind _slots (Variables|Item|GetSlots))
  (bind _item (Utilities|Array|Get(acopy) _slots Index))
  (if (and (not (Inventory|IsSlotEmpty? Index)) (<= (+ (Item|GetAmountatIndex Index) Amount) (Variables|Item|GetMaxStackSize)))
    (Utilities|Array|SetArrayElem _slots Index (Utilities|Struct|MakeS_InventorySlot (.itemclass _item) (+ (.amount _item) Amount)))
    (CallFunction|UpdateSlotatIndex Index)
    (return true)
    (else
      (return false))))

(fn ShowStorage
  (bind _returnvalue (Game|GetPlayerController 0))
  (Widget|SetVisibility (Variables|Default|GetStorageWidget) "Visible")
  (Input|SetInputModeGameandUI _returnvalue 0 "DoNotLock" true)
  (Variables|/Script/Engine.PlayerController|SetbShowMouseCursor _returnvalue true)
  (Variables|/Game/InventorySystem/Blueprints/BP_Inventory.BP_Inventory_C|SetStorageOpen? (Variables|/Game/Game/Character/Player/Ch_MyCharacter.Ch_MyCharacter_C|GetInventoryRef (Variables|Default|GetMyCharacterRef)) true))

(fn HideStorage
  (bind _returnvalue (Game|GetPlayerController 0))
  (Widget|SetVisibility (Variables|Default|GetStorageWidget) "Hidden")
  (Input|SetInputModeGameOnly _returnvalue)
  (Variables|/Script/Engine.PlayerController|SetbShowMouseCursor _returnvalue false)
  (Variables|/Game/InventorySystem/Blueprints/BP_Inventory.BP_Inventory_C|SetStorageOpen? (Variables|/Game/Game/Character/Player/Ch_MyCharacter.Ch_MyCharacter_C|GetInventoryRef (Variables|Default|GetMyCharacterRef)) false))

(fn MovefromInvtoStorIndex
  (params (Inventory :type BP%20Inventory%20Object%20Reference) (Inventoryindex :type Integer) (StorageIndex :type Integer))
  (LocalVariables|SetLocalInventory Inventory)
  (LocalVariables|SetLocalInvIndex Inventoryindex)
  (LocalVariables|SetLocalStorIndex StorageIndex)
  (if (Inventory|IsSlotEmpty? (LocalVariables|GetLocalStorIndex))
    (LocalVariables|SetAmountToAdd (Default|GetAmountatIndex (LocalVariables|GetLocalInventory) (LocalVariables|GetLocalInvIndex)))
    (bind _success_ (CallFunction|AddItemtoIndex (LocalVariables|GetLocalStorIndex) (.ItemClass (Utilities|Struct|BreakS_InventorySlot (Utilities|Array|Get(acopy) (Variables|/Game/InventorySystem/Blueprints/BP_Inventory.BP_Inventory_C|GetSlots (LocalVariables|GetLocalInventory)) (LocalVariables|GetLocalInvIndex)))) (LocalVariables|GetAmountToAdd)))
    (if _success_
      (Default|RemoveItematIndex (LocalVariables|GetLocalInventory) (LocalVariables|GetLocalInvIndex) (LocalVariables|GetAmountToAdd))
      (return true)
      (else
        (return false)))
    (elif (Math|Boolean|ANDBoolean (== (.ItemClass (Utilities|Struct|BreakS_InventorySlot (Utilities|Array|Get(acopy) (Variables|Item|GetSlots) (LocalVariables|GetLocalStorIndex)))) (.ItemClass (Utilities|Struct|BreakS_InventorySlot (Utilities|Array|Get(acopy) (Variables|/Game/InventorySystem/Blueprints/BP_Inventory.BP_Inventory_C|GetSlots (LocalVariables|GetLocalInventory)) (LocalVariables|GetLocalInvIndex))))) (.CanBeStacked? (Utilities|Struct|BreakS_ItemInfo (.ItemInfo (Item|GetItemInfoatIndex (LocalVariables|GetLocalStorIndex))))) (< (Item|GetAmountatIndex (LocalVariables|GetLocalStorIndex)) (Variables|Item|GetMaxStackSize)))
      (LocalVariables|SetAmountToAdd (Math|Integer|SelectInt (- (Variables|Item|GetMaxStackSize) (Item|GetAmountatIndex (LocalVariables|GetLocalStorIndex))) (Default|GetAmountatIndex (LocalVariables|GetLocalInventory) (LocalVariables|GetLocalInvIndex)) (> (Default|GetAmountatIndex (LocalVariables|GetLocalInventory) (LocalVariables|GetLocalInvIndex)) (- (Variables|Item|GetMaxStackSize) (Item|GetAmountatIndex (LocalVariables|GetLocalStorIndex))))))
      (bind _success__2 (CallFunction|IncreaseAmountatIndex (LocalVariables|GetLocalStorIndex) (LocalVariables|GetAmountToAdd)))
      (if _success__2
        (Default|RemoveItematIndex (LocalVariables|GetLocalInventory) (LocalVariables|GetLocalInvIndex) (LocalVariables|GetAmountToAdd))
        (return true)
        (else
          (return false)))
      (else
        (return false)))))

(fn MooveAlltoInventory
  (params (Inventory :type BP%20Inventory%20Object%20Reference))
  (bind _output_get (LocalVariables|SetLocalInv Inventory))
  (Utilities|IsValid _output_get
    (:Is%20Valid
      (for (_array_element _array_index) (Variables|Item|GetSlots)
        (if (Utilities|IsValidClass (.ItemClass (Utilities|Struct|BreakS_InventorySlot _array_element)))
          (bind (_success_ _rest) (Default|AddItem (LocalVariables|GetLocalInv) (.ItemClass (Utilities|Struct|BreakS_InventorySlot _array_element)) (.Amount (Utilities|Struct|BreakS_InventorySlot _array_element)) false))
          (if _success_
            (Item|RemoveItematIndex _array_index (- (.Amount (Utilities|Struct|BreakS_InventorySlot _array_element)) _rest)))))
      (return))
    (:Is%20Not%20Valid
      (return))))