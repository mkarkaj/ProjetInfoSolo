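; Merchant actor that offers a shop to the player character within the inventory system.
; A sphere overlap registers it as the character's NearbyMerchant and toggles its prompt text.
; OnInteract, guarded by a DoOnce, opens a centered ShopWidget, refreshes the inventory, flags the shop open and freezes movement.
; OnShopClosed restores walking, refreshes a visible inventory, removes the widget and resets the guard.
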(event OnComponentBeginOverlap(Sphere)
  (params (OverlappedComponent :type Primitive%20Component%20Object%20Reference) (OtherActor :type Actor%20Object%20Reference) (OtherComp :type Primitive%20Component%20Object%20Reference) (OtherBodyIndex :type Integer) (bFromSweep :type Boolean) (SweepResult :type Hit%20Result%20Structure%20%28by%20ref%29))
  (bind _asch_my_character (Utilities|Casting|CastToCh_MyCharacter OtherActor))
  (Variables|/Game/Game/Character/Player/Ch_MyCharacter.Ch_MyCharacter_C|SetNearbyMerchant _asch_my_character self)
  (Rendering|SetVisibility (Variables|Default|GetMerchantText) true false))

(event OnComponentEndOverlap(Sphere)
  (params (OverlappedComponent :type Primitive%20Component%20Object%20Reference) (OtherActor :type Actor%20Object%20Reference) (OtherComp :type Primitive%20Component%20Object%20Reference) (OtherBodyIndex :type Integer))
  (bind _asch_my_character (Utilities|Casting|CastToCh_MyCharacter OtherActor))
  (Variables|/Game/Game/Character/Player/Ch_MyCharacter.Ch_MyCharacter_C|SetNearbyMerchant _asch_my_character 0)
  (Rendering|SetVisibility (Variables|Default|GetMerchantText) false false))

(event Custom|OnInteract
  (params (MyCharacter :type Ch%20My%20Character%20Object%20Reference))
  (Utilities|FlowControl|DoOnce false
    (:Completed
      (Variables|Default|SetMyCharacter MyCharacter)
      (bind _returnvalue (UserInterface|CreateWidget "/Game/InventorySystem/Widgets/ShopWidget.ShopWidget_C" 0 self (Variables|Default|GetMyCharacter)))
      (Variables|Default|SetShopWidget _returnvalue)
      (Class|UserWidget|SetPositioninViewport :self (Variables|Default|GetShopWidget) :bRemoveDPIScale false)
      (Class|UserWidget|SetAnchorsinViewport (Variables|Default|GetShopWidget) (Utilities|Struct|MakeAnchors "(X=0.500000,Y=0.500000)" "(X=0.500000,Y=0.500000)"))
      (Class|UserWidget|SetAlignmentinViewport (Variables|Default|GetShopWidget) "(X=0.500000,Y=0.500000)")
      (UserInterface|Viewport|AddtoViewport (Variables|Default|GetShopWidget) 5)
      (Default|HideInventory (Variables|/Game/Game/Character/Player/Ch_MyCharacter.Ch_MyCharacter_C|GetInventoryRef (Variables|Default|GetMyCharacter)))
      (Default|ShowInventory (Variables|/Game/Game/Character/Player/Ch_MyCharacter.Ch_MyCharacter_C|GetInventoryRef (Variables|Default|GetMyCharacter)))
      (Variables|/Game/Game/Character/Player/Ch_MyCharacter.Ch_MyCharacter_C|SetIsShopOpen? (Variables|Default|GetMyCharacter) true)
      (Pawn|Components|CharacterMovement|DisableMovement (Variables|/Script/Engine.Character|GetCharacterMovement (Variables|Default|GetMyCharacter)))
      (Components|Movement|StopMovementImmediately (Variables|/Script/Engine.Character|GetCharacterMovement (Variables|Default|GetMyCharacter))))))

(event Custom|OnShopClosed
  (Variables|/Game/Game/Character/Player/Ch_MyCharacter.Ch_MyCharacter_C|SetIsShopOpen? (Variables|Default|GetMyCharacter) false)
  (Pawn|Components|CharacterMovement|SetMovementMode (Variables|/Script/Engine.Character|GetCharacterMovement (Variables|Default|GetMyCharacter)) "MOVE_Walking" 0)
  (if (Variables|/Game/InventorySystem/Blueprints/BP_Inventory.BP_Inventory_C|GetIsVisible? (Variables|/Game/Game/Character/Player/Ch_MyCharacter.Ch_MyCharacter_C|GetInventoryRef (Variables|Default|GetMyCharacter)))
    (Default|HideInventory (Variables|/Game/Game/Character/Player/Ch_MyCharacter.Ch_MyCharacter_C|GetInventoryRef (Variables|Default|GetMyCharacter)))
    (Default|ShowInventory (Variables|/Game/Game/Character/Player/Ch_MyCharacter.Ch_MyCharacter_C|GetInventoryRef (Variables|Default|GetMyCharacter))))
  (Widget|RemovefromParent (Variables|Default|GetShopWidget))
  (Variables|Default|SetShopWidget 0)
  (Utilities|FlowControl|DoOnce false) ; enters at Reset
)

(fn ConstructionScript)