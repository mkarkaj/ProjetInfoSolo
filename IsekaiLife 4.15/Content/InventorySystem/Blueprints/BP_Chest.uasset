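; BP_Chest is an interactable chest that gives the player a storage inventory, optionally filled with random starting loot.
; On BeginPlay it can roll each data table row's chance and amount to build StartItems.
; Its overlap range toggles prompt text and registers it as the character's NearbyChest.
; Interaction, gated by DoOnce, lazily spawns and shows BP_Storage and freezes movement; closing restores walking and resets the gate.
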(event OnComponentBeginOverlap(InteractionRange)
  (params (OverlappedComponent :type Primitive%20Component%20Object%20Reference) (OtherActor :type Actor%20Object%20Reference) (OtherComp :type Primitive%20Component%20Object%20Reference) (OtherBodyIndex :type Integer) (bFromSweep :type Boolean) (SweepResult :type Hit%20Result%20Structure%20%28by%20ref%29))
  (bind _asch_my_character (Utilities|Casting|CastToCh_MyCharacter OtherActor))
  (Rendering|SetVisibility (Variables|Default|GetChestText) true false)
  (Variables|/Game/Game/Character/Player/Ch_MyCharacter.Ch_MyCharacter_C|SetNearbyChest _asch_my_character self))

(event OnComponentEndOverlap(InteractionRange)
  (params (OverlappedComponent :type Primitive%20Component%20Object%20Reference) (OtherActor :type Actor%20Object%20Reference) (OtherComp :type Primitive%20Component%20Object%20Reference) (OtherBodyIndex :type Integer))
  (bind _asch_my_character (Utilities|Casting|CastToCh_MyCharacter OtherActor))
  (Rendering|SetVisibility (Variables|Default|GetChestText) false false)
  (Variables|/Game/Game/Character/Player/Ch_MyCharacter.Ch_MyCharacter_C|SetNearbyChest _asch_my_character 0))

(event Custom|OnStorageClosed
  (Default|HideStorage (Variables|Default|GetStorageActor))
  (Pawn|Components|CharacterMovement|SetMovementMode (Variables|/Script/Engine.Character|GetCharacterMovement (Variables|Default|GetMyCharacter)) "MOVE_Walking" 0)
  (if (Variables|/Game/InventorySystem/Blueprints/BP_Inventory.BP_Inventory_C|GetIsVisible? (Variables|/Game/Game/Character/Player/Ch_MyCharacter.Ch_MyCharacter_C|GetInventoryRef (Variables|Default|GetMyCharacter)))
    (Default|HideInventory (Variables|/Game/Game/Character/Player/Ch_MyCharacter.Ch_MyCharacter_C|GetInventoryRef (Variables|Default|GetMyCharacter)))
    (Default|ShowInventory (Variables|/Game/Game/Character/Player/Ch_MyCharacter.Ch_MyCharacter_C|GetInventoryRef (Variables|Default|GetMyCharacter)))
    (Utilities|FlowControl|DoOnce false) ; enters at Reset
    (else
      (Utilities|FlowControl|DoOnce false) ; enters at Reset
    )))

(event Custom|OnInteract
  (params (MyCharacter :type Ch%20My%20Character%20Object%20Reference))
  (Utilities|FlowControl|DoOnce false
    (:Completed
      (Variables|Default|SetMyCharacter MyCharacter)
      (Utilities|IsValid (Variables|Default|GetStorageActor)
        (:Is%20Valid
          _)
        (:Is%20Not%20Valid
          (bind _returnvalue (Game|SpawnActorfromClass "/Game/InventorySystem/Blueprints/BP_Storage.BP_Storage_C" (Math|Transform|MakeTransform "0, 0, 0" "0, 0, 0" "1,1,1") "AlwaysSpawn" 0 (Variables|Default|GetAmoundOfSlots) (Variables|Default|GetMyCharacter) (Variables|Default|GetSlotsPerRow) self (Variables|Default|GetStartItems)))
          (Variables|Default|SetStorageActor _returnvalue)))
      (Default|GenerateSlotWidgets (Variables|/Game/InventorySystem/Blueprints/BP_Storage.BP_Storage_C|GetStorageWidget (Variables|Default|GetStorageActor)) (Variables|Default|GetStorageActor))
      (Default|ShowStorage (Variables|Default|GetStorageActor))
      (Default|HideInventory (Variables|/Game/Game/Character/Player/Ch_MyCharacter.Ch_MyCharacter_C|GetInventoryRef (Variables|Default|GetMyCharacter)))
      (Default|ShowInventory (Variables|/Game/Game/Character/Player/Ch_MyCharacter.Ch_MyCharacter_C|GetInventoryRef (Variables|Default|GetMyCharacter)))
      (Pawn|Components|CharacterMovement|DisableMovement (Variables|/Script/Engine.Character|GetCharacterMovement (Variables|Default|GetMyCharacter)))
      (Components|Movement|StopMovementImmediately (Variables|/Script/Engine.Character|GetCharacterMovement (Variables|Default|GetMyCharacter))))))

(event EventBeginPlay
  (if (Variables|Default|GetGenerateStartItems?)
    (CallFunction|GenerateStartItems)))

(fn ConstructionScript)

(fn GenerateStartItems
  (bind _outrownames (DataTable|GetDataTableRowNames "/Game/InventorySystem/Blueprints/DataTables/Table_ChestStartItems.Table_ChestStartItems"))
  (for _array_element _outrownames
    (bind _returnvalue (Utilities|GetDataTableRow "/Game/InventorySystem/Blueprints/DataTables/Table_ChestStartItems.Table_ChestStartItems" _array_element)
      (:then
        (if (and (Utilities|IsValidClass (.ItemClass (Utilities|Struct|BreakS_ChestContent _returnvalue))) (<= (Math|Random|RandomIntegerinRange 1 100) (.Chance (Utilities|Struct|BreakS_ChestContent _returnvalue))))
          (Utilities|Array|Add (Variables|Default|GetStartItems) (Utilities|Struct|MakeS_InventorySlot (.ItemClass (Utilities|Struct|BreakS_ChestContent _returnvalue)) (Math|Random|RandomIntegerinRange (.MinimumAmount (Utilities|Struct|BreakS_ChestContent _returnvalue)) (.MaximumAmount (Utilities|Struct|BreakS_ChestContent _returnvalue)))))))))
  (return))