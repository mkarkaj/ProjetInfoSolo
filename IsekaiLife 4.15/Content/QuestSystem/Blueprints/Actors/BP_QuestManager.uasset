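; Quest manager actor that adds, selects, ends and cancels quests, syncing the quest list and journal widgets and granting gold, experience and regional prestige on completion.
; Kill, item-found and NPC-talk events advance matching sub-goals, deferring quest-completing ones to avoid changing quest arrays mid-loop.
; The selected sub-goal spawns a location marker that drives distance text and a minimap arrow as the player moves.
; NPCs cached at BeginPlay let cancellations notify quest clients.
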(event Custom|OnSwitchSubQuest
  (bind _currentquest (Variables|Default|GetCurrentQuest))
  (bind _mainwidget (Variables|Default|GetMainWidget))
  (Utilities|IsValid (Variables|Default|GetCurrentGoalActor)
    (:Is%20Valid
      (Actor|DestroyActor (Variables|Default|GetCurrentGoalActor)))
    (:Is%20Not%20Valid
      _))
  (bind _output_get (Variables|Default|SetCurrentSubGoal (Utilities|Array|Get(acopy) (.SubGoals (Utilities|Struct|BreakS_QuestInfo (Variables|/Game/QuestSystem/Blueprints/Actors/QuestActors/BP_MasterQuest.BP_MasterQuest_C|GetQuestInfo _currentquest))) (Variables|/Game/QuestSystem/Blueprints/Actors/QuestActors/BP_MasterQuest.BP_MasterQuest_C|GetSelectedSubGoalIndex _currentquest))))
  (if (.HasLocation (Utilities|Struct|BreakS_GoalLocation (.GoalLocation (Utilities|Struct|BreakS_GoalInfo _output_get))))
    (bind _returnvalue (Game|SpawnActorfromClass "/Game/QuestSystem/Blueprints/Actors/BP_GoalActor.BP_GoalActor_C" (Math|Transform|MakeTransform (.Location (Utilities|Struct|BreakS_GoalLocation (.GoalLocation (Utilities|Struct|BreakS_GoalInfo _output_get)))) "0, 0, 0" "1,1,1") "AlwaysSpawn" 0 (.UseRadius? (Utilities|Struct|BreakS_GoalInfo _output_get)) (.Radius (Utilities|Struct|BreakS_GoalInfo _output_get)) (.CircleColor (Utilities|Struct|BreakS_GoalInfo _output_get))))
    (Variables|Default|SetCurrentGoalActor _returnvalue)
    (bind _output_get_2 (Variables|Default|SetCurrentDistance (CallFunction|DistancetoGoal)))
    (Rendering|Components|TextRender|SetText (Variables|/Game/Game/Widget/MainWidget.MainWidget_C|GetDistanceText (Variables|Default|GetMainWidget)) (Utilities|Text|ToText(Integer) _output_get_2 false))
    (CallFunction|UpdateDirectionArrow)
    (Widget|SetVisibility (Variables|/Game/Game/Widget/MainWidget.MainWidget_C|GetDistanceBorder _mainwidget) "HitTestInvisible")
    (Widget|SetVisibility (Variables|/Game/QuestSystem/Widgets/MiniMap.MiniMap_C|GetDirectionArrow (Variables|/Game/Game/Widget/MainWidget.MainWidget_C|GetMiniMap_132 _mainwidget)) (select (>= (Variables|Default|GetCurrentDistance) (Variables|Default|GetShowDirectionArrowAmount)) "HitTestInvisible" "Hidden"))
    (else
      (Variables|Default|SetCurrentGoalActor 0)
      (Widget|SetVisibility (Variables|/Game/Game/Widget/MainWidget.MainWidget_C|GetDistanceBorder (Variables|Default|GetMainWidget)) "Hidden"))))

(event Custom|OnTalkedToNpc
  (params (NpcClass :type Master%20NPC%20Class%20Reference) (NpcId :type Integer))
  (Utilities|Array|Clear (Variables|Default|GetIndiceToCompleteLater))
  (for _array_element (Variables|Default|GetCurrentQuestActors)
    (for (_array_element_2 _array_index) (Variables|/Game/QuestSystem/Blueprints/Actors/QuestActors/BP_MasterQuest.BP_MasterQuest_C|GetCurrentGoals _array_element)
      (if (Math|Boolean|ANDBoolean (Utilities|Enum|Equal(Enum) (.Type (Utilities|Struct|BreakS_GoalInfo _array_element_2)) "NewEnumerator3") (== (.GoalClass (Utilities|Struct|BreakS_GoalInfo _array_element_2)) NpcClass) (== (.GoalId (Utilities|Struct|BreakS_GoalInfo _array_element_2)) NpcId))
        (if (.CompletesQuest? (Utilities|Struct|BreakS_GoalInfo _array_element_2))
          (Utilities|Array|Add (Variables|Default|GetIndiceToCompleteLater) (Utilities|Struct|MakeS_IndexToComplete _array_element (Utilities|Array|Get(acopy) (Variables|/Game/QuestSystem/Blueprints/Actors/QuestActors/BP_MasterQuest.BP_MasterQuest_C|GetCurrentGoalIndices _array_element) _array_index)))
          (else
            (Default|CompleteSubGoal _array_element (Utilities|Array|Get(acopy) (Variables|/Game/QuestSystem/Blueprints/Actors/QuestActors/BP_MasterQuest.BP_MasterQuest_C|GetCurrentGoalIndices _array_element) _array_index) false)))))
    (CallFunction|CompleateGoals)))

(event Custom|OnPlayerMove
  (Utilities|IsValid (Variables|Default|GetCurrentGoalActor)
    (:Is%20Valid
      (bind _output_get (Variables|Default|SetCurrentDistance (CallFunction|DistancetoGoal)))
      (Rendering|Components|TextRender|SetText (Variables|/Game/Game/Widget/MainWidget.MainWidget_C|GetDistanceText (Variables|Default|GetMainWidget)) (Utilities|Text|ToText(Integer) _output_get))
      (Math|Integer|CompareInt (Variables|Default|GetCurrentDistance) (Variables|Default|GetShowDirectionArrowAmount)
        (:>
          _)
        (:==
          _)
        (:<
          (Utilities|FlowControl|DoOnce false :!label _label
            (:Completed
              (Widget|SetVisibility (Variables|/Game/QuestSystem/Widgets/MiniMap.MiniMap_C|GetDirectionArrow (Variables|/Game/Game/Widget/MainWidget.MainWidget_C|GetMiniMap_132 (Variables|Default|GetMainWidget))) "Hidden")
              (goto _label_2 Reset)))))
      (CallFunction|UpdateDirectionArrow)
      (Utilities|FlowControl|DoOnce false :!label _label_2
        (:Completed
          (Widget|SetVisibility (Variables|/Game/QuestSystem/Widgets/MiniMap.MiniMap_C|GetDirectionArrow (Variables|/Game/Game/Widget/MainWidget.MainWidget_C|GetMiniMap_132 (Variables|Default|GetMainWidget))) "HitTestInvisible")
          (goto _label Reset))))))

(event Custom|OnEnemyKilled
  (params (Class :type Master%20Enemy%20Class%20Reference))
  (Utilities|Array|Clear (Variables|Default|GetIndiceToCompleteLater))
  (Variables|Default|SetKillEnemy Class)
  (for _array_element (Variables|Default|GetCurrentQuestActors)
    (for (_array_element_2 _array_index) (Variables|/Game/QuestSystem/Blueprints/Actors/QuestActors/BP_MasterQuest.BP_MasterQuest_C|GetCurrentGoals _array_element)
      (if (and (Utilities|Enum|Equal(Enum) (.Type (Utilities|Struct|BreakS_GoalInfo _array_element_2)) "NewEnumerator1") (== (.GoalClass (Utilities|Struct|BreakS_GoalInfo _array_element_2)) (Variables|Default|GetKillEnemy)))
        (if (>= (+ (Utilities|Array|Get(acopy) (Variables|/Game/QuestSystem/Blueprints/Actors/QuestActors/BP_MasterQuest.BP_MasterQuest_C|GetCurrentHuntedAmounts _array_element) _array_index) 1) (.AmountToHunt (Utilities|Struct|BreakS_GoalInfo _array_element_2)))
          (if (.CompletesQuest? (Utilities|Struct|BreakS_GoalInfo _array_element_2))
            (Utilities|Array|Add (Variables|Default|GetIndiceToCompleteLater) (Utilities|Struct|MakeS_IndexToComplete _array_element (Utilities|Array|Get(acopy) (Variables|/Game/QuestSystem/Blueprints/Actors/QuestActors/BP_MasterQuest.BP_MasterQuest_C|GetCurrentGoalIndices _array_element) _array_index)))
            (else
              (Default|CompleteSubGoal _array_element (Utilities|Array|Get(acopy) (Variables|/Game/QuestSystem/Blueprints/Actors/QuestActors/BP_MasterQuest.BP_MasterQuest_C|GetCurrentGoalIndices _array_element) _array_index) false)))
          (else
            (Utilities|Array|SetArrayElem (Variables|/Game/QuestSystem/Blueprints/Actors/QuestActors/BP_MasterQuest.BP_MasterQuest_C|GetCurrentHuntedAmounts _array_element) _array_index (+ (Utilities|Array|Get(acopy) (Variables|/Game/QuestSystem/Blueprints/Actors/QuestActors/BP_MasterQuest.BP_MasterQuest_C|GetCurrentHuntedAmounts _array_element) _array_index) 1))
            (Default|Update (Utilities|Array|Get(acopy) (Variables|/Game/QuestSystem/Widgets/QuestWidget.QuestWidget_C|GetSubGoalWidgets (Variables|/Game/QuestSystem/Blueprints/Actors/QuestActors/BP_MasterQuest.BP_MasterQuest_C|GetQuestWidget _array_element)) _array_index))
            (if (Default|SelectedinJournal? _array_element)
              (Default|GenerateSubGoals (Variables|/Game/Game/Widget/MainWidget.MainWidget_C|GetJournal (Variables|Default|GetMainWidget)))))))))
  (CallFunction|CompleateGoals))

(event Custom|OnItemFound
  (params (FoundItem :type BP%20Master%20Item%20Class%20Reference))
  (Utilities|Array|Clear (Variables|Default|GetIndiceToCompleteLater))
  (Variables|Default|SetFoundObject FoundItem)
  (for _array_element (Variables|Default|GetCurrentQuestActors)
    (for (_array_element_2 _array_index) (Variables|/Game/QuestSystem/Blueprints/Actors/QuestActors/BP_MasterQuest.BP_MasterQuest_C|GetCurrentGoals _array_element)
      (if (and (Utilities|Enum|Equal(Enum) (.Type (Utilities|Struct|BreakS_GoalInfo _array_element_2)) "NewEnumerator2") (== (.GoalClass (Utilities|Struct|BreakS_GoalInfo _array_element_2)) (Variables|Default|GetFoundObject)))
        (if (.CompletesQuest? (Utilities|Struct|BreakS_GoalInfo _array_element_2))
          (Utilities|Array|Add (Variables|Default|GetIndiceToCompleteLater) (Utilities|Struct|MakeS_IndexToComplete _array_element (Utilities|Array|Get(acopy) (Variables|/Game/QuestSystem/Blueprints/Actors/QuestActors/BP_MasterQuest.BP_MasterQuest_C|GetCurrentGoalIndices _array_element) _array_index)))
          (else
            (Default|CompleteSubGoal _array_element (Utilities|Array|Get(acopy) (Variables|/Game/QuestSystem/Blueprints/Actors/QuestActors/BP_MasterQuest.BP_MasterQuest_C|GetCurrentGoalIndices _array_element) _array_index) false))))))
  (CallFunction|CompleateGoals))

(event EventBeginPlay
  (CallFunction|GetAllNpcs))

(fn ConstructionScript)

(fn SelectNewQuest
  (params (Quest :type BP%20Master%20Quest%20Object%20Reference) (SubGoal :type Sub%20Goal%20Widget%20Object%20Reference))
  (Utilities|IsValid (Variables|Default|GetCurrentQuest)
    (:Is%20Valid
      (Widget|SetIsEnabled (Variables|/Game/QuestSystem/Widgets/QuestWidget.QuestWidget_C|GetQuestName (Variables|/Game/QuestSystem/Blueprints/Actors/QuestActors/BP_MasterQuest.BP_MasterQuest_C|GetQuestWidget (Variables|Default|GetCurrentQuest))) false)
      (Default|SelectSubGoal (Variables|/Game/QuestSystem/Blueprints/Actors/QuestActors/BP_MasterQuest.BP_MasterQuest_C|GetQuestWidget (Variables|Default|GetCurrentQuest))))
    (:Is%20Not%20Valid
      _))
  (bind _output_get (Variables|Default|SetCurrentQuest Quest))
  (Default|OnQuestSelected (Variables|/Game/QuestSystem/Blueprints/Actors/QuestActors/BP_MasterQuest.BP_MasterQuest_C|GetQuestWidget _output_get) SubGoal)
  (return))

(fn AddNewQuest
  (params (QuestClass :type BP%20Master%20Quest%20Class%20Reference) (DirectlyStart? :type Boolean))
  (bind _mainwidget (Variables|Default|GetMainWidget))
  (LocalVariables|SetlocalClass QuestClass)
  (LocalVariables|SetLocalStart DirectlyStart?)
  (if (and (Utilities|IsValidClass QuestClass) (not (Utilities|Array|ContainsItem (Variables|Default|GetAllQuestClasses) QuestClass)))
    (Utilities|Array|Add (Variables|Default|GetAllQuestClasses) (LocalVariables|GetlocalClass))
    (bind _returnvalue (Game|SpawnActorfromClass (LocalVariables|GetlocalClass) (Math|Transform|MakeTransform "0, 0, 0" "0, 0, 0" "1,1,1") "AlwaysSpawn" 0 self 0))
    (bind _output_get (LocalVariables|SetLocalQuestActor _returnvalue))
    (Utilities|Array|Add (Variables|Default|GetCurrentQuestActors) _output_get)
    (bind _widget (Default|AddQUesttoList (Variables|Default|GetMainWidget) (LocalVariables|GetLocalQuestActor)))
    (bind _output_get_2 (Variables|/Game/QuestSystem/Blueprints/Actors/QuestActors/BP_MasterQuest.BP_MasterQuest_C|SetQuestWidget (LocalVariables|GetLocalQuestActor) _widget))
    (Default|SetUpStartingGoals (LocalVariables|GetLocalQuestActor))
    (Default|UpdateQuest _output_get_2)
    (Default|AddEntry (Variables|/Game/Game/Widget/MainWidget.MainWidget_C|GetJournal (Variables|Default|GetMainWidget)) (LocalVariables|GetLocalQuestActor))
    (if (or (LocalVariables|GetLocalStart) (<= (Utilities|Array|Length (Variables|Default|GetCurrentQuestActors)) 1))
      (CallFunction|SelectNewQuest (LocalVariables|GetLocalQuestActor) (Utilities|Array|Get(acopy) (Variables|/Game/QuestSystem/Widgets/QuestWidget.QuestWidget_C|GetSubGoalWidgets (Variables|/Game/QuestSystem/Blueprints/Actors/QuestActors/BP_MasterQuest.BP_MasterQuest_C|GetQuestWidget (LocalVariables|GetLocalQuestActor))))))
    (if (Variables|/Game/Game/Widget/MainWidget.MainWidget_C|GetSlideOut? (Variables|Default|GetMainWidget))
      (UserInterface|Animation|PlayAnimation _mainwidget (Variables|/Game/Game/Widget/MainWidget.MainWidget_C|GetSlideOut _mainwidget) 0.0 1 "Reverse" 1.0)
      (Variables|/Game/Game/Widget/MainWidget.MainWidget_C|SetSlideOut? _mainwidget false)
      (return true)
      (else
        (return true)))
    (else
      (return false))))

(fn DistancetoGoal
  (bind _currentgoalactor (Variables|Default|GetCurrentGoalActor))
  (bind _character (Variables|Default|GetCharacter))
  (bind _returnvalue (Transformation|GetActorLocation _character))
  (bind _returnvalue_2 (Transformation|GetActorLocation _currentgoalactor))
  (return (Math|Float|Round (/ (Math|Vector|VectorLength (- (Math|Vector|MakeVector (.x _returnvalue) (.y _returnvalue) 0.0) (Math|Vector|MakeVector (.x _returnvalue_2) (.y _returnvalue_2) 0.0))) 1e+02))))

(fn UpdateDirectionArrow
  (Class|Widget|SetRenderAngle (Variables|/Game/QuestSystem/Widgets/MiniMap.MiniMap_C|GetDirectionArrow (Variables|/Game/Game/Widget/MainWidget.MainWidget_C|GetMiniMap_132 (Variables|Default|GetMainWidget))) (.Yaw (Math|Rotator|BreakRotator (Math|Rotator|FindLookatRotation (Transformation|GetActorLocation (Variables|Default|GetCharacter)) (Transformation|GetActorLocation (Variables|Default|GetCurrentGoalActor))))))
  (return))

(fn HasCurrentQuest?
  (params (QuestClass :type BP%20Master%20Quest%20Class%20Reference))
  (bind _array_element (Utilities|Array|ForEachLoopwithBreak (Variables|Default|GetCurrentQuestActors) :!label _label)
    (:LoopBody
      (if (== (Utilities|GetClass _array_element) QuestClass)
        (LocalVariables|SetFoundQuest _array_element)
        (goto _label Break)))
    (:Completed
      (Utilities|IsValid (LocalVariables|GetFoundQuest)
        (:Is%20Valid
          (return true (LocalVariables|GetFoundQuest)))
        (:Is%20Not%20Valid
          (return false 0))))))

(fn EndQuest
  (params (Quest :type BP%20Master%20Quest%20Object%20Reference))
  (bind _currentgoalactor (Variables|Default|GetCurrentGoalActor))
  (bind _completedquestactors (Variables|Default|GetCompletedQuestActors))
  (bind _character (Variables|Default|GetCharacter))
  (bind _item (Utilities|Array|Get(acopy) _completedquestactors))
  (bind _output_get (LocalVariables|SetLocalQuest Quest))
  (Utilities|Array|RemoveItem (Variables|Default|GetCurrentQuestActors) _output_get)
  (Utilities|Array|Add (Utilities|Select :Index (Variables|/Game/QuestSystem/Blueprints/Actors/QuestActors/BP_MasterQuest.BP_MasterQuest_C|GetCurrentState (LocalVariables|GetLocalQuest)) :NewEnumerator0 (Variables|Default|GetCurrentQuestActors) :NewEnumerator1 (Variables|Default|GetCompletedQuestActors) :NewEnumerator2 (Variables|Default|GetFailedQuestActors)) (LocalVariables|GetLocalQuest))
  (Default|AddEntry (Variables|/Game/Game/Widget/MainWidget.MainWidget_C|GetJournal (Variables|Default|GetMainWidget)) (LocalVariables|GetLocalQuest))
  (if (== (LocalVariables|GetLocalQuest) (Variables|Default|GetCurrentQuest))
    (Variables|Default|SetCurrentQuest 0)
    (Utilities|IsValid _currentgoalactor
      (:Is%20Valid
        (Actor|DestroyActor _currentgoalactor)
        (Widget|SetVisibility (Variables|/Game/Game/Widget/MainWidget.MainWidget_C|GetDistanceBorder (Variables|Default|GetMainWidget)) "Hidden"))
      (:Is%20Not%20Valid
        _))
    (Utilities|IsValid _item
      (:Is%20Valid
        (CallFunction|SelectNewQuest _item (Utilities|Array|Get(acopy) (Variables|/Game/QuestSystem/Widgets/QuestWidget.QuestWidget_C|GetSubGoalWidgets (Variables|/Game/QuestSystem/Blueprints/Actors/QuestActors/BP_MasterQuest.BP_MasterQuest_C|GetQuestWidget _item)))))
      (:Is%20Not%20Valid
        _)))
  (if (Default|SelectedinJournal? (LocalVariables|GetLocalQuest))
    (Default|OnQuestClicked (Variables|/Game/Game/Widget/MainWidget.MainWidget_C|GetJournal (Variables|Default|GetMainWidget))))
  (if (Utilities|Enum|Equal(Enum) (Variables|/Game/QuestSystem/Blueprints/Actors/QuestActors/BP_MasterQuest.BP_MasterQuest_C|GetCurrentState (LocalVariables|GetLocalQuest)) "NewEnumerator1")
    (Default|IncreaseGold _character (.Monney (Utilities|Struct|BreakS_QuestReward (.ComplitionReward (Utilities|Struct|BreakS_QuestInfo (Variables|/Game/QuestSystem/Blueprints/Actors/QuestActors/BP_MasterQuest.BP_MasterQuest_C|GetQuestInfo (LocalVariables|GetLocalQuest)))))))
    (Default|AddExpPoints _character (.Experience (Utilities|Struct|BreakS_QuestReward (.ComplitionReward (Utilities|Struct|BreakS_QuestInfo (Variables|/Game/QuestSystem/Blueprints/Actors/QuestActors/BP_MasterQuest.BP_MasterQuest_C|GetQuestInfo (LocalVariables|GetLocalQuest)))))))
    (Default|SetPrestigebyRegion _character (.Region (Utilities|Struct|BreakS_QuestInfo (Variables|/Game/QuestSystem/Blueprints/Actors/QuestActors/BP_MasterQuest.BP_MasterQuest_C|GetQuestInfo (LocalVariables|GetLocalQuest)))) (+ (Default|GetPrestigebyRegion _character (.Region (Utilities|Struct|BreakS_QuestInfo (Variables|/Game/QuestSystem/Blueprints/Actors/QuestActors/BP_MasterQuest.BP_MasterQuest_C|GetQuestInfo (LocalVariables|GetLocalQuest))))) (.PrestigePoints (Utilities|Struct|BreakS_QuestReward (.ComplitionReward (Utilities|Struct|BreakS_QuestInfo (Variables|/Game/QuestSystem/Blueprints/Actors/QuestActors/BP_MasterQuest.BP_MasterQuest_C|GetQuestInfo (LocalVariables|GetLocalQuest))))))))
    (return)
    (else
      (return))))

(fn CompleateGoals
  (for _array_element (Variables|Default|GetIndiceToCompleteLater)
    (Default|CompleteSubGoal (.Quest (Utilities|Struct|BreakS_IndexToComplete _array_element)) (.Index (Utilities|Struct|BreakS_IndexToComplete _array_element)) false)))

(fn GetAllNpcs
  (bind _outactors (Actor|GetAllActorsOfClass "/Game/QuestSystem/Blueprints/Character/Master_NPC.Master_NPC_C"))
  (Variables|Default|SetAllNpcInWorld _outactors)
  (return))

(fn FindNpcbyId
  (params (Class :type Master%20NPC%20Class%20Reference) (Id :type Integer))
  (bind _array_element (Utilities|Array|ForEachLoopwithBreak (Variables|Default|GetAllNpcInWorld) :!label _label)
    (:LoopBody
      (if (and (== (Utilities|GetClass _array_element) Class) (== (Variables|/Game/QuestSystem/Blueprints/Character/Master_NPC.Master_NPC_C|GetNpcId _array_element) Id))
        (Variables|Default|SetlocalFoundNpc _array_element)
        (goto _label Break)))
    (:Completed
      (Utilities|IsValid (Variables|Default|GetlocalFoundNpc)
        (:Is%20Valid
          (return true (Variables|Default|GetlocalFoundNpc)))
        (:Is%20Not%20Valid
          (return false 0))))))

(fn CancelQuest
  (params (QuestRef :type BP%20Master%20Quest%20Object%20Reference))
  (bind _currentgoalactor (Variables|Default|GetCurrentGoalActor))
  (bind _completedquestactors (Variables|Default|GetCompletedQuestActors))
  (bind _item (Utilities|Array|Get(acopy) _completedquestactors))
  (bind _output_get (LocalVariables|SetLocalQuest QuestRef))
  (Utilities|Array|RemoveItem (Variables|Default|GetCurrentQuestActors) _output_get)
  (if (== (LocalVariables|GetLocalQuest) (Variables|Default|GetCurrentQuest))
    (Variables|Default|SetCurrentQuest 0)
    (Utilities|IsValid _currentgoalactor
      (:Is%20Valid
        (Actor|DestroyActor _currentgoalactor)
        (Widget|SetVisibility (Variables|/Game/Game/Widget/MainWidget.MainWidget_C|GetDistanceBorder (Variables|Default|GetMainWidget)) "Hidden"))
      (:Is%20Not%20Valid
        _))
    (Utilities|IsValid _item
      (:Is%20Valid
        (CallFunction|SelectNewQuest _item (Utilities|Array|Get(acopy) (Variables|/Game/QuestSystem/Widgets/QuestWidget.QuestWidget_C|GetSubGoalWidgets (Variables|/Game/QuestSystem/Blueprints/Actors/QuestActors/BP_MasterQuest.BP_MasterQuest_C|GetQuestWidget _item)))))
      (:Is%20Not%20Valid
        _)))
  (if (Default|SelectedinJournal? (LocalVariables|GetLocalQuest))
    (Default|OnQuestClicked (Variables|/Game/Game/Widget/MainWidget.MainWidget_C|GetJournal (Variables|Default|GetMainWidget))))
  (if (.HasClient? (Utilities|Struct|BreakS_QuestInfo (Variables|/Game/QuestSystem/Blueprints/Actors/QuestActors/BP_MasterQuest.BP_MasterQuest_C|GetQuestInfo (LocalVariables|GetLocalQuest))))
    (bind (_found_ _npc) (CallFunction|FindNpcbyId (.ClientClass (Utilities|Struct|BreakS_QuestInfo (Variables|/Game/QuestSystem/Blueprints/Actors/QuestActors/BP_MasterQuest.BP_MasterQuest_C|GetQuestInfo (LocalVariables|GetLocalQuest)))) (.ClientId (Utilities|Struct|BreakS_QuestInfo (Variables|/Game/QuestSystem/Blueprints/Actors/QuestActors/BP_MasterQuest.BP_MasterQuest_C|GetQuestInfo (LocalVariables|GetLocalQuest))))))
    (if _found_
      (Default|OnOwnQuestCancelled _npc (Utilities|GetClass (LocalVariables|GetLocalQuest)))))
  (Utilities|Array|RemoveItem (Variables|Default|GetAllQuestClasses) (Utilities|GetClass (LocalVariables|GetLocalQuest)))
  (Actor|DestroyActor (LocalVariables|GetLocalQuest))
  (return))