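; BP_MasterQuest is the base quest actor that tracks one quest's active, completed and failed sub-goals and its evolving description.
; CompleteSubGoal records each result, then ends the quest through QuestManager or activates the following goals, exposing completion and failure events.
; AddGoalForIndex creates sub-goal widgets, or recursively auto-completes goals whose required item is already in the inventory.
; It also keeps the journal in sync and removes its widgets on cancel or end.
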(event Custom|OnGoalCompleted
  (params (GoalIndex :type Integer)))

(event Custom|OnGoalFailed
  (params (GoalIndex :type Integer)))

(event Custom|OnQuestCancel
  (CallFunction|RemoveWidgets)
  (Default|CancelQuest (Variables|DoNotTouch!|GetQuestManager) self))

(event EventBeginPlay)

(event Collision|EventActorBeginOverlap
  (params (OtherActor :type Actor%20Object%20Reference)))

(event EventTick
  (params (DeltaSeconds :type Float%20%28single-precision%29)))

(fn ConstructionScript)

(fn UpdateSubGoals
  (Utilities|Array|Clear (Variables|DoNotTouch!|GetCurrentGoals))
  (for _array_element (Variables|DoNotTouch!|GetCurrentGoalIndices)
    (Utilities|Array|Add (Variables|DoNotTouch!|GetCurrentGoals) (Utilities|Array|Get(acopy) (.SubGoals (Utilities|Struct|BreakS_QuestInfo (Variables|QuestInformation|GetQuestInfo))) _array_element)))
  (return))

(fn SetUpStartingGoals
  (Utilities|Array|Clear (Variables|DoNotTouch!|GetCurrentGoalIndices))
  (Variables|DoNotTouch!|SetCurrentDescription (.Description (Utilities|Struct|BreakS_QuestInfo (Variables|QuestInformation|GetQuestInfo))))
  (for _array_element (Variables|QuestInformation|GetStartingSubGoalIndices)
    (CallFunction|AddGoalforIndex _array_element))
  (Utilities|Array|Resize (Variables|DoNotTouch!|GetCurrentHuntedAmounts) (Utilities|Array|Length (Variables|DoNotTouch!|GetCurrentGoalIndices)))
  (CallFunction|UpdateSubGoals)
  (return))

(fn GotoNextSubGoal
  (bind _currentgoalindices (Variables|DoNotTouch!|GetCurrentGoalIndices))
  (bind _currentgoalindices_2 (Variables|DoNotTouch!|GetCurrentGoalIndices))
  (bind _maxvalue (Math|Integer|MaxOfIntArray _currentgoalindices))
  (bind _returnvalue (+ _maxvalue 1))
  (if (<= _returnvalue (Utilities|Array|LastIndex (.SubGoals (Utilities|Struct|BreakS_QuestInfo (Variables|QuestInformation|GetQuestInfo)))))
    (LocalVariables|SetNextIndex _returnvalue)
    (Utilities|Array|Clear _currentgoalindices_2)
    (Utilities|Array|Add _currentgoalindices_2 (LocalVariables|GetNextIndex))
    (CallFunction|UpdateSubGoals)
    (return true)
    (else
      (return false))))

(fn CompleteSubGoal
  (params (SubGoalIndex :type Integer) (Fail? :type Boolean))
  (bind _currentgoalindices (Variables|DoNotTouch!|GetCurrentGoalIndices))
  (bind _questwidget (Variables|DoNotTouch!|GetQuestWidget))
  (bind _questwidget_2 (Variables|DoNotTouch!|GetQuestWidget))
  (bind _subgoalwidgets (Variables|/Game/QuestSystem/Widgets/QuestWidget.QuestWidget_C|GetSubGoalWidgets _questwidget))
  (LocalVariables|SetLocalFail Fail?)
  (LocalVariables|SetLocalSubGoalIndex SubGoalIndex)
  (if (Utilities|Array|ContainsItem (Variables|DoNotTouch!|GetCurrentGoalIndices) (LocalVariables|GetLocalSubGoalIndex))
    (bind _output_get (LocalVariables|SetLocalCompletedGoal (Utilities|Array|Get(acopy) (.SubGoals (Utilities|Struct|BreakS_QuestInfo (Variables|QuestInformation|GetQuestInfo))) (LocalVariables|GetLocalSubGoalIndex))))
    (Utilities|Array|Add (Variables|DoNotTouch!|GetCompletedSubGoal) (Utilities|Struct|MakeS_CompletedGoal (LocalVariables|GetLocalSubGoalIndex) _output_get (not (LocalVariables|GetLocalFail))))
    (if (and (.UpdateQuestDescription? (Utilities|Struct|BreakS_GoalInfo (LocalVariables|GetLocalCompletedGoal))) (not (LocalVariables|GetLocalFail)))
      (Variables|DoNotTouch!|SetCurrentDescription (Utilities|Text|FormatText "{Current} {next}" (Variables|DoNotTouch!|GetCurrentDescription) (.UpdatedDescription (Utilities|Struct|BreakS_GoalInfo (LocalVariables|GetLocalCompletedGoal)))))
      (if (CallFunction|SelectedinJournal?)
        (Default|UpdateDescription (Variables|/Game/Game/Widget/MainWidget.MainWidget_C|GetJournal (Variables|/Game/QuestSystem/Blueprints/Actors/BP_QuestManager.BP_QuestManager_C|GetMainWidget (Variables|DoNotTouch!|GetQuestManager))))))
    (Utilities|Array|RemoveItem (Variables|DoNotTouch!|GetCurrentGoals) (LocalVariables|GetLocalCompletedGoal))
    (LocalVariables|SetLocalWidgetIndex (Utilities|Array|FindItem _currentgoalindices (LocalVariables|GetLocalSubGoalIndex)))
    (Utilities|Array|RemoveIndex (Variables|DoNotTouch!|GetCurrentHuntedAmounts) (Utilities|Array|FindItem _currentgoalindices (LocalVariables|GetLocalSubGoalIndex)))
    (Utilities|Array|RemoveItem _currentgoalindices (LocalVariables|GetLocalSubGoalIndex))
    (Widget|RemovefromParent (Utilities|Array|Get(acopy) _subgoalwidgets (LocalVariables|GetLocalWidgetIndex)))
    (Utilities|Array|RemoveIndex _subgoalwidgets (LocalVariables|GetLocalWidgetIndex))
    (if (LocalVariables|GetLocalFail)
      (CallFunction|OnGoalFailed (LocalVariables|GetLocalSubGoalIndex))
      (if (.FailMeansQuestFail? (Utilities|Struct|BreakS_GoalInfo (LocalVariables|GetLocalCompletedGoal)))
        _
        (else
          (if (CallFunction|SelectedinJournal?) :!label _label
            (Default|GenerateSubGoals (Variables|/Game/Game/Widget/MainWidget.MainWidget_C|GetJournal (Variables|/Game/QuestSystem/Blueprints/Actors/BP_QuestManager.BP_QuestManager_C|GetMainWidget (Variables|DoNotTouch!|GetQuestManager)))))
          (if (and (== (LocalVariables|GetLocalSubGoalIndex) (Variables|DoNotTouch!|GetSelectedSubGoalIndex)) (== (Variables|/Game/QuestSystem/Blueprints/Actors/BP_QuestManager.BP_QuestManager_C|GetCurrentQuest (Variables|DoNotTouch!|GetQuestManager)) self))
            (Default|SelectSubGoal _questwidget_2 (Utilities|Array|Get(acopy) (Variables|/Game/QuestSystem/Widgets/QuestWidget.QuestWidget_C|GetSubGoalWidgets _questwidget_2))))
          (return true)))
      (else
        (CallFunction|OnGoalCompleted (LocalVariables|GetLocalSubGoalIndex))
        (if (.CompletesQuest? (Utilities|Struct|BreakS_GoalInfo (LocalVariables|GetLocalCompletedGoal)))
          _
          (else
            (for _array_element (.FollowingSubGoalIndices (Utilities|Struct|BreakS_GoalInfo (LocalVariables|GetLocalCompletedGoal)))
              (CallFunction|AddGoalforIndex _array_element))
            (goto _label)))))
    (for (_array_element_2 _array_index) (Variables|DoNotTouch!|GetCurrentGoalIndices)
      (Utilities|Array|Add (Variables|DoNotTouch!|GetCompletedSubGoal) (Utilities|Struct|MakeS_CompletedGoal _array_element_2 (CallFunction|GoalatIndex _array_index) false)))
    (Utilities|Array|Clear (Variables|DoNotTouch!|GetCurrentGoalIndices))
    (Utilities|Array|Clear (Variables|DoNotTouch!|GetCurrentHuntedAmounts))
    (Utilities|Array|Clear (Variables|DoNotTouch!|GetCurrentGoals))
    (Variables|DoNotTouch!|SetCurrentState (select (LocalVariables|GetLocalFail) "NewEnumerator2" "NewEnumerator1"))
    (CallFunction|RemoveWidgets)
    (Default|EndQuest (Variables|DoNotTouch!|GetQuestManager) self)
    (return true)
    (else
      (return false))))

(fn SelectedinJournal?
  (bind _questmanager (Variables|DoNotTouch!|GetQuestManager))
  (bind _mainwidget (Variables|/Game/QuestSystem/Blueprints/Actors/BP_QuestManager.BP_QuestManager_C|GetMainWidget _questmanager))
  (bind _journal (Variables|/Game/Game/Widget/MainWidget.MainWidget_C|GetJournal _mainwidget))
  (bind _selectedquest (Variables|/Game/QuestSystem/Widgets/QuestJournal.QuestJournal_C|GetSelectedQuest _journal))
  (return (and (Utilities|IsValid _selectedquest) (== _selectedquest self))))

(fn GoalatIndex
  (params (Index :type Integer))
  (return (Utilities|Array|Get(acopy) (.SubGoals (Utilities|Struct|BreakS_QuestInfo (Variables|QuestInformation|GetQuestInfo))) Index)))

(fn GoalAlreadyFound?
  (params (GoalIndex :type Integer))
  (bind _goalinfo (CallFunction|GoalatIndex GoalIndex))
  (bind (_type _customgoal_ _goaltext _additionalname _amounttohunt _goalclass) (Utilities|Struct|BreakS_GoalInfo _goalinfo))
  (if (Utilities|Enum|Equal(Enum) _type "NewEnumerator2")
    (bind _array_element (Utilities|Array|ForEachLoopwithBreak (Variables|/Game/InventorySystem/Blueprints/BP_Inventory.BP_Inventory_C|GetSlots (Variables|/Game/Game/Character/Player/Ch_MyCharacter.Ch_MyCharacter_C|GetInventoryRef (Variables|/Game/QuestSystem/Blueprints/Actors/BP_QuestManager.BP_QuestManager_C|GetCharacter (Variables|DoNotTouch!|GetQuestManager)))) :!label _label)
      (:LoopBody
        (if (== (.ItemClass (Utilities|Struct|BreakS_InventorySlot _array_element)) _goalclass)
          (LocalVariables|SetLocalBool true)
          (goto _label Break)))
      (:Completed
        (return (LocalVariables|GetLocalBool))))
    (else
      (return false))))

(fn AddGoalforIndex
  (params (Index :type Integer))
  (bind _questwidget (Variables|DoNotTouch!|GetQuestWidget))
  (bind _output_get (LocalVariables|SetLocalIndex Index))
  (if (CallFunction|GoalAlreadyFound? _output_get)
    (Utilities|Array|Add (Variables|DoNotTouch!|GetCompletedSubGoal) (Utilities|Struct|MakeS_CompletedGoal (LocalVariables|GetLocalIndex) (CallFunction|GoalatIndex (LocalVariables|GetLocalIndex)) true))
    (CallFunction|OnGoalCompleted (LocalVariables|GetLocalIndex))
    (if (.UpdateQuestDescription? (Utilities|Struct|BreakS_GoalInfo (CallFunction|GoalatIndex (LocalVariables|GetLocalIndex))))
      (Variables|DoNotTouch!|SetCurrentDescription (Utilities|Text|FormatText "{Current} {next}" (Variables|DoNotTouch!|GetCurrentDescription) (.UpdatedDescription (Utilities|Struct|BreakS_GoalInfo (CallFunction|GoalatIndex (LocalVariables|GetLocalIndex))))))
      (if (CallFunction|SelectedinJournal?)
        (Default|UpdateDescription (Variables|/Game/Game/Widget/MainWidget.MainWidget_C|GetJournal (Variables|/Game/QuestSystem/Blueprints/Actors/BP_QuestManager.BP_QuestManager_C|GetMainWidget (Variables|DoNotTouch!|GetQuestManager))))))
    (for _array_element (.FollowingSubGoalIndices (Utilities|Struct|BreakS_GoalInfo (CallFunction|GoalatIndex (LocalVariables|GetLocalIndex))))
      (CallFunction|AddGoalforIndex _array_element))
    (return)
    (else
      (bind _returnvalue (Utilities|Array|Add (Variables|DoNotTouch!|GetCurrentGoalIndices) (LocalVariables|GetLocalIndex)))
      (if (> _returnvalue (Utilities|Array|LastIndex (Variables|DoNotTouch!|GetCurrentHuntedAmounts)))
        (Utilities|Array|Add (Variables|DoNotTouch!|GetCurrentHuntedAmounts) 0))
      (Utilities|Array|Add (Variables|DoNotTouch!|GetCurrentGoals) (CallFunction|GoalatIndex (LocalVariables|GetLocalIndex)))
      (bind _returnvalue_2 (UserInterface|CreateWidget "/Game/QuestSystem/Widgets/sUBgOALwIDGET.SubGoalWidget_C" 0 (CallFunction|GoalatIndex (LocalVariables|GetLocalIndex)) self (Variables|DoNotTouch!|GetQuestWidget)))
      (Utilities|Array|Add (Variables|/Game/QuestSystem/Widgets/QuestWidget.QuestWidget_C|GetSubGoalWidgets _questwidget) _returnvalue_2)
      (Widget|Panel|AddChild (Variables|/Game/QuestSystem/Widgets/QuestWidget.QuestWidget_C|GetSubgoalBox _questwidget) _returnvalue_2)
      (return))))

(fn RemoveWidgets
  (bind _questmanager (Variables|DoNotTouch!|GetQuestManager))
  (bind _listenterwidget (Variables|DoNotTouch!|GetListEnterWidget))
  (bind _mainwidget (Variables|/Game/QuestSystem/Blueprints/Actors/BP_QuestManager.BP_QuestManager_C|GetMainWidget _questmanager))
  (Utilities|Array|RemoveItem (Variables|/Game/Game/Widget/MainWidget.MainWidget_C|GetQuestWidget _mainwidget) (Variables|DoNotTouch!|GetQuestWidget))
  (Utilities|Array|RemoveItem (Variables|/Game/QuestSystem/Widgets/QuestJournal.QuestJournal_C|GetAllQuestEntries (Variables|/Game/Game/Widget/MainWidget.MainWidget_C|GetJournal _mainwidget)) _listenterwidget)
  (Widget|RemovefromParent _listenterwidget))