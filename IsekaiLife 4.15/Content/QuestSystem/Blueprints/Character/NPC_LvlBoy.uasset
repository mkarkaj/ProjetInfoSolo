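; NPC_LvlBoy is a quest-giving NPC whose quest unlocks once the player reaches a required level.
; On player level-up it checks the level requirement, then flags the quest as available and shows its quest mark.
; Interacting then adds and starts the quest through the character's quest manager, hides the mark and changes its default message.
; Interactions outside that one-time offer fall through to the parent class behavior.
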(event EventBeginPlay
  (|CallParentFunction))

(event Collision|EventActorBeginOverlap
  (params (OtherActor :type Actor%20Object%20Reference)))

(event EventTick
  (params (DeltaSeconds :type Float%20%28single-precision%29)))

(event EventOnPlayerLevelUp
  (params (NewLevel :type Integer))
  (if (Math|Boolean|ANDBoolean (>= NewLevel (Variables|Default|GetRequiredLvl)) (not (Variables|Default|GetCanGiveQuest?)) (not (Variables|Default|GetHasGivenQuest?)))
    (Variables|Default|SetCanGiveQuest? true)
    (Rendering|SetVisibility (Variables|Default|GetQuestMark) true false)))

(event EventOnInteractwith
  (params (Character :type Ch%20My%20Character%20Object%20Reference))
  (if (and (Variables|Default|GetCanGiveQuest?) (not (Variables|Default|GetHasGivenQuest?)))
    (Default|AddNewQuest (Variables|/Game/Game/Character/Player/Ch_MyCharacter.Ch_MyCharacter_C|GetQuestManagerRef Character) (Variables|Default|GetQuestToGive) true)
    (Variables|Default|SetHasGivenQuest? true)
    (Variables|Default|SetDefaultMsg "Good Job! You have grown up !!")
    (Rendering|SetVisibility (Variables|Default|GetQuestMark) false false)
    (else
      (|CallParentFunction Character))))

(fn ConstructionScript
  (|CallParentFunction))