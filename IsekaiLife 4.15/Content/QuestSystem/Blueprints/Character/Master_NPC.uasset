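; Base NPC for the quest system that hands out an optional quest or shows a timed dialogue message.
; Interacting starts an unowned quest through the player's quest manager and hides the quest mark, which returns on cancellation.
; Otherwise it displays its default message and reports the conversation to the quest manager.
; Player radius events toggle the interaction prompt, and optional patrolling loops through target points via AIMoveTo.
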(event Custom|MoveToCurrentPatrolPoint
  ;[1 1 1] Move to the next partrolePoint in the array
  (AI|AIMoveTo self (Transformation|GetActorLocation (Utilities|Array|Get(acopy) (Variables|Default|GetPatrollingPoints) (Variables|Default|GetCurrentPatrolIndex))) 0 4e+01 true
    (:OnSuccess
      (Variables|Default|SetCurrentPatrolIndex (select (< (Variables|Default|GetCurrentPatrolIndex) (Utilities|Array|LastIndex (Variables|Default|GetPatrollingPoints))) (+ (Variables|Default|GetCurrentPatrolIndex) 1) 0))
      (CallFunction|MovetoCurrentPatrolPoint))))

(event Custom|OnOwnQuestCancelled
  (params (QuestClass :type BP%20Master%20Quest%20Class%20Reference))
  (Rendering|SetVisibility (Variables|Default|GetQuestMark) true false))

(event Custom|OnPlayerLevelUp
  (params (NewLevel :type Integer)))

(event Custom|OnPlayerGainPrestige
  (params (Player :type Ch%20My%20Character%20Object%20Reference)))

(event Custom|OnTalkedTo
  (params (Player :type Ch%20My%20Character%20Object%20Reference))
  ;[1 1 1] On talked to
  (CallFunction|ShowMessage (Variables|Default|GetDefaultMsg) (Variables|Default|GetDefaultDuration) Player))

(event Custom|ShowMessage
  (params (Message :type Text) (Duration :type Float%20%28single-precision%29) (Player :type Ch%20My%20Character%20Object%20Reference))
  ;[1 1 1] ShowMessage
  (if (Variables|Default|GetCanBeTalkedTo?)
    (Variables|Default|SetCanBeTalkedTo? true)
    (Rendering|SetVisibility (Variables|Default|GetInteractionWidget) false false)
    (Rendering|Components|TextRender|SetText (Variables|/Game/QuestSystem/Widgets/MessageWidget.MessageWidget_C|GetMessage (Variables|Default|GetMessageWidget)) Message)
    (Rendering|SetVisibility (Variables|Default|GetMessageComponent) true false)
    (Default|OnTalkedtoNpc (Variables|/Game/Game/Character/Player/Ch_MyCharacter.Ch_MyCharacter_C|GetQuestManagerRef Player) (Utilities|GetClass self) (Variables|Default|GetNpcId))
    (Utilities|FlowControl|Delay Duration)
    (Rendering|SetVisibility (Variables|Default|GetMessageComponent) false false)
    (Rendering|SetVisibility (Variables|Default|GetInteractionWidget) (Variables|Default|GetInPlayerRadius?) false)
    (Variables|Default|SetCanBeTalkedTo? true)))

(event EventBeginPlay
  ;[1 1 1] Event Begin play
  (Actor|SetOwner (Game|GetPlayerCharacter 0))
  (Rendering|SetVisibility (Variables|Default|GetQuestMark) (Utilities|IsValidClass (Variables|Default|GetHasQuest)) false)
  (Variables|Default|SetMessageWidget (.AsMessage%20Widget (Utilities|Casting|CastToMessageWidget (UserInterface|GetUserWidgetObject (Variables|Default|GetMessageComponent)))))
  (bind _asinteract_text (Utilities|Casting|CastToInteractText (UserInterface|GetUserWidgetObject (Variables|Default|GetInteractionWidget)))
    (:then
      (Rendering|Components|TextRender|SetText (Variables|/Game/QuestSystem/Widgets/InteractText.InteractText_C|GetNameText _asinteract_text) (Variables|Default|GetName)))
    (:CastFailed
      _))
  (if (and (Variables|Default|GetDoesPatrol?) (> (Utilities|Array|Length (Variables|Default|GetPatrollingPoints)) 0))
    (CallFunction|MovetoCurrentPatrolPoint)))

(event EventOnEnterPlayerRadius
  (params (Character :type Ch%20My%20Character%20Object%20Reference))
  ;[1 1 1] On enter/leave player radius
  (Variables|Default|SetInPlayerRadius? true)
  (if (Variables|Default|GetCanBeTalkedTo?)
    (Rendering|SetVisibility (Variables|Default|GetInteractionWidget) true false)))

(event EventOnLeavePlayerRadius
  (params (Character :type Ch%20My%20Character%20Object%20Reference))
  ;[1 1 1] On enter/leave player radius
  (Variables|Default|SetInPlayerRadius? false)
  (Rendering|SetVisibility (Variables|Default|GetInteractionWidget) false false))

(event EventOnInteractwith
  (params (Character :type Ch%20My%20Character%20Object%20Reference))
  (bind _questmanagerref (Variables|/Game/Game/Character/Player/Ch_MyCharacter.Ch_MyCharacter_C|GetQuestManagerRef Character))
  (bind _hasquest (Variables|Default|GetHasQuest))
  ;[1 1 1] On interact with
  (if (Utilities|IsValidClass _hasquest)
    (if (Utilities|Array|ContainsItem (Variables|/Game/QuestSystem/Blueprints/Actors/BP_QuestManager.BP_QuestManager_C|GetAllQuestClasses _questmanagerref) _hasquest)
      (CallFunction|OnTalkedto Character)
      (else
        (Default|AddNewQuest _questmanagerref (Variables|Default|GetHasQuest) true)
        (Rendering|SetVisibility (Variables|Default|GetQuestMark) false false)))
    (else
      (CallFunction|OnTalkedto Character))))

(fn ConstructionScript)